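; Blueprint for a spinning platform generator that rotates a platform through a RotatingMovement component.
; On BeginPlay it picks a random spin direction and sets the yaw rate from the game mode's level and speed multiplier.
; It binds to the RzGameMode OnSpeedChanged event and recomputes the rotation rate whenever that fires, keeping the same direction.
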(event `self.ReceiveBeginPlay`
  (bind _asrz_game_mode (cast `/Game/RZFallGuys/Blueprints/RzGameMode` (`GameplayStatics.GetGameMode`)))
  (set `self.Direction` (`KismetMathLibrary.RandomIntegerInRange` 0 1))
  (add `/Game/RZFallGuys/Blueprints/RzGameMode.OnSpeedChanged` _asrz_game_mode (delegate `OnSpeedChanged_Event_0`))
  (set `RotatingMovementComponent.RotationRate` (`KismetMathLibrary.MakeRotator` 0.0 0.0 (* (* (- (* (`self.Direction`) 2) 1) (+ (* (`/Game/RZFallGuys/Blueprints/RzGameMode.Level` _asrz_game_mode) 10.0) 55.0)) (`/Game/RZFallGuys/Blueprints/RzGameMode.SpeedMultiplier` _asrz_game_mode))) (`self.RotatingMovement`) :!label _label))

(event `OnSpeedChanged_Event_0`
  (params (`Speed Modifier` :type "Float (double-precision)"))
  (goto _label))

(fn `UserConstructionScript`)