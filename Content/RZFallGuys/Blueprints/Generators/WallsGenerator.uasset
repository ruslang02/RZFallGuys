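; Generator actor that scatters a random number of Wall obstacles around its location when play begins.
; The RzGameMode Level caps the wall count and raises wall height.
; Each wall gets a randomized XY position, shifted by a fixed offset, and a random Y scale.
; Spawned walls are tracked in DynamicActors and destroyed along with the generator.
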(event `self.ReceiveDestroyed`
  (bind _dynamicactors (`self.DynamicActors`))
  (for _array_element _dynamicactors
    (`self.K2_DestroyActor` _array_element))
  (`KismetArrayLibrary.Array_Clear` _dynamicactors))

(event `self.ReceiveBeginPlay`
  (bind _returnvalue (`KismetMathLibrary.RandomFloatInRange` 1.0 5.0))
  (bind _returnvalue_2 (- 500.0 (* 100.0 _returnvalue)))
  (bind _asrz_game_mode (cast `/Game/RZFallGuys/Blueprints/RzGameMode` (`GameplayStatics.GetGameMode`)))
  (bind _level (`/Game/RZFallGuys/Blueprints/RzGameMode.Level` _asrz_game_mode))
  (for _ (range 1 (+ (`KismetMathLibrary.RandomIntegerInRange` 1 _level) 1))
    (bind _returnvalue_3 (`|SpawnActorFromClass` "/Game/RZFallGuys/Blueprints/Generators/Wall.Wall_C" (`KismetMathLibrary.MakeTransform` (+ (`KismetMathLibrary.MakeVector` (+ (`KismetMathLibrary.RandomFloatInRange` -450.0 450.0) (.x (`self.K2_GetActorLocation`))) (+ (`KismetMathLibrary.RandomFloatInRange` (* _returnvalue_2 -1.0) _returnvalue_2) (.y (`self.K2_GetActorLocation`)))) (500.0 500.0 10.0)) (struct) (`KismetMathLibrary.MakeVector` 1.0 _returnvalue (+ (* _level 0.05) 0.9))) "Undefined" "OverrideRootScale" null null))
    (`KismetArrayLibrary.Array_Add` (`self.DynamicActors`) _returnvalue_3)))

(fn `UserConstructionScript`)