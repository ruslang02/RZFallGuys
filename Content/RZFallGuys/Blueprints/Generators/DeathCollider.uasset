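; DeathCollider is a moving hazard cube that fails the level when the player pawn overlaps it.
; Tick slides Cube1 back and forth along local Y, reversing at fixed limits, with speed scaled by RzGameMode's level and speed multiplier.
; It binds to the game mode's passthrough-changed event, which turns off the cube's collision and swaps in a semi-transparent danger material while passthrough is active.
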(event `self.ReceiveTick`
  (params (DeltaSeconds :type "Float (single-precision)"))
  (bind _asrz_game_mode (cast `/Game/RZFallGuys/Blueprints/RzGameMode` (`GameplayStatics.GetGameMode`)))
  (bind _returnvalue (* (`/Game/RZFallGuys/Blueprints/RzGameMode.SpeedMultiplier` _asrz_game_mode) (`self.Direction`) DeltaSeconds (+ (* (`/Game/RZFallGuys/Blueprints/RzGameMode.Level` _asrz_game_mode) 75.0) 500.0)))
  (bind _output_get (set `self.CurrentPosition` (+ (`self.CurrentPosition`) _returnvalue)))
  (`SceneComponent.K2_SetRelativeLocation` (`self.Cube1`) (+ (`KismetMathLibrary.MakeVector` 0.0 _returnvalue) (`SceneComponent.RelativeLocation` (`self.Cube1`))) false false)
  (if (> _output_get 2300.0)
    (set `self.Direction` -1.0)
    (elif (< _output_get 0.0)
      (set `self.Direction` 1.0))))

(event `self.ReceiveBeginPlay`
  (bind _asrz_game_mode (cast `/Game/RZFallGuys/Blueprints/RzGameMode` (`GameplayStatics.GetGameMode`)))
  (add `/Game/RZFallGuys/Blueprints/RzGameMode.OnPassthroughChanged` _asrz_game_mode (delegate `OnPassthroughChanged`)))

(event `OnPassthroughChanged`
  (params (IsPassthrough :type Boolean))
  (bind _cube1 (`self.Cube1`))
  (bind _cube1_2 (`self.Cube1`))
  (if IsPassthrough
    (`PrimitiveComponent.SetCollisionEnabled` _cube1 "NoCollision")
    (`PrimitiveComponent.SetMaterial` _cube1_2 0 "/Game/RZFallGuys/Assets/CubeDangerSemiTransparentMaterial.CubeDangerSemiTransparentMaterial")
    (else
      (`PrimitiveComponent.SetCollisionEnabled` _cube1 "QueryAndPhysics")
      (`PrimitiveComponent.SetMaterial` _cube1_2 0 "/Game/RZFallGuys/Assets/CubeDangerMaterial.CubeDangerMaterial"))))

(event `self.Cube1.OnComponentBeginOverlap`
  (params (OverlappedComponent :type "PrimitiveComponent Object Reference") (OtherActor :type "Actor Object Reference") (OtherComp :type "PrimitiveComponent Object Reference") (OtherBodyIndex :type Integer) (bFromSweep :type Boolean) (SweepResult :type "HitResult Structure (by ref)"))
  (if (== OtherActor (`GameplayStatics.GetPlayerPawn` 0))
    (bind _asrz_game_mode (cast `/Game/RZFallGuys/Blueprints/RzGameMode` (`GameplayStatics.GetGameMode`)))
    (`/Game/RZFallGuys/Blueprints/RzGameMode.FailLevel` _asrz_game_mode)))

(fn `UserConstructionScript`)