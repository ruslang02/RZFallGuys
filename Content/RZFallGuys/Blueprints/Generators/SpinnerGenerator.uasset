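; SpinnerGenerator is a spinning obstacle that rotates around yaw in a randomly chosen direction.
; On BeginPlay it binds to RzGameMode events and sets its RotatingMovement rate, which grows with the current level and scales with the speed multiplier.
; Speed changes recompute that rate.
; Passthrough changes toggle collision and swap between solid and semi-transparent materials on all its static meshes.
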(event `OnSpeedChanged`
  (params (`Speed Modifier` :type "Float (double-precision)"))
  (set `RotatingMovementComponent.RotationRate` (`KismetMathLibrary.MakeRotator` 0.0 0.0 (* (`/Game/RZFallGuys/Blueprints/RzGameMode.SpeedMultiplier` (stale `self.ReceiveBeginPlay` _asrz_game_mode)) (* (- (* (`self.Direction`) 2) 1) (+ (* (`/Game/RZFallGuys/Blueprints/RzGameMode.Level` (stale `self.ReceiveBeginPlay` _asrz_game_mode)) 9.0) 60.0)))) (`self.RotatingMovement`) :!label _label))

(event `self.ReceiveBeginPlay`
  (bind _asrz_game_mode (cast `/Game/RZFallGuys/Blueprints/RzGameMode` (`GameplayStatics.GetGameMode`)))
  (set `self.Direction` (`KismetMathLibrary.RandomIntegerInRange` 0 1))
  (add `/Game/RZFallGuys/Blueprints/RzGameMode.OnPassthroughChanged` _asrz_game_mode (delegate `OnPassthroughChanged`))
  (add `/Game/RZFallGuys/Blueprints/RzGameMode.OnSpeedChanged` _asrz_game_mode (delegate `OnSpeedChanged`))
  (goto _label))

(event `OnPassthroughChanged`
  (params (IsPassthrough :type Boolean))
  (for _array_element (`self.K2_GetComponentsByClass` "/Script/Engine.StaticMeshComponent")
    (if IsPassthrough
      (`PrimitiveComponent.SetCollisionEnabled` _array_element "NoCollision")
      (`PrimitiveComponent.SetMaterial` _array_element 0 "/Game/RZFallGuys/Assets/CubeSemiTransparentMaterial.CubeSemiTransparentMaterial")
      (else
        (`PrimitiveComponent.SetCollisionEnabled` _array_element "QueryAndPhysics")
        (`PrimitiveComponent.SetMaterial` _array_element 0 "/Game/RZFallGuys/Assets/CubeMaterial.CubeMaterial")))))

(fn `UserConstructionScript`)