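; Wall Blueprint whose cube switches between solid and passthrough as the RzGameMode passthrough state changes.
; Tick binds the change handler to the game mode each frame, rather than once at BeginPlay.
; Passthrough disables collision and applies a semi-transparent material.
; Turning it off restores both, first teleporting an overlapping player pawn to a fixed raised relative location rather than offsetting it.
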(event `self.ReceiveTick`
  (params (DeltaSeconds :type "Float (single-precision)"))
  (bind _asrz_game_mode (cast `/Game/RZFallGuys/Blueprints/RzGameMode` (`GameplayStatics.GetGameMode`)))
  (add `/Game/RZFallGuys/Blueprints/RzGameMode.OnPassthroughChanged` _asrz_game_mode (delegate `OnPassthroughChanged`)))

(event `OnPassthroughChanged`
  (params (IsPassthrough :type Boolean))
  (bind _returnvalue (`GameplayStatics.GetPlayerPawn` 0))
  (bind _cube (`self.Cube`))
  (if IsPassthrough
    (`PrimitiveComponent.SetCollisionEnabled` _cube "NoCollision")
    (`PrimitiveComponent.SetMaterial` _cube 0 "/Game/RZFallGuys/Assets/CubeSemiTransparentMaterial.CubeSemiTransparentMaterial")
    (else
      (if (`PrimitiveComponent.IsOverlappingActor` _cube _returnvalue)
        (`self.K2_SetActorRelativeLocation` _returnvalue (0.0 0.0 300.0) false true))
      (`PrimitiveComponent.SetCollisionEnabled` _cube "QueryAndPhysics")
      (`PrimitiveComponent.SetMaterial` _cube 0 "/Game/RZFallGuys/Assets/CubeMaterial.CubeMaterial"))))

(fn `UserConstructionScript`)