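; EndingPlatform is the goal platform that finishes the level when the player reaches it.
; When the player pawn overlaps its Box, it turns off the box's overlap events and calls FinishLevel on the RzGameMode.
; Tick re-enables overlap events whenever the platform's location changes, so the finish trigger re-arms after the platform is moved.
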(event `self.Box.OnComponentBeginOverlap`
  (params (OverlappedComponent :type "PrimitiveComponent Object Reference") (OtherActor :type "Actor Object Reference") (OtherComp :type "PrimitiveComponent Object Reference") (OtherBodyIndex :type Integer) (bFromSweep :type Boolean) (SweepResult :type "HitResult Structure (by ref)"))
  (bind _asrz_game_mode (cast `/Game/RZFallGuys/Blueprints/RzGameMode` (`GameplayStatics.GetGameMode`)))
  (if (== (`GameplayStatics.GetPlayerPawn` 0) OtherActor)
    (set `PrimitiveComponent.bGenerateOverlapEvents` false (`self.Box`))
    (`/Game/RZFallGuys/Blueprints/RzGameMode.FinishLevel` _asrz_game_mode)))

(event `self.ReceiveTick`
  (params (DeltaSeconds :type "Float (single-precision)"))
  (bind _returnvalue (`self.K2_GetActorLocation`))
  (if (not (== (`self.PreviousLocation`) _returnvalue))
    (set `PrimitiveComponent.bGenerateOverlapEvents` true (`self.Box`))
    (set `self.PreviousLocation` _returnvalue)))

(fn `UserConstructionScript`)