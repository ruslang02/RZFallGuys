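; GamePlatform is a level platform that fills its grid of 1000-unit cells with randomly chosen generator actors at BeginPlay.
; An integer bitmap tracks occupancy: each spawn takes the lowest free bit, and its bounds mark the cells it covers.
; Grid size comes from Width and the actor's X scale.
; Spawned actors are stored in Platforms and destroyed along with this actor.
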(event `self.ReceiveDestroyed`
  (bind _platforms (`self.Platforms`))
  (for _array_element _platforms
    (`self.K2_DestroyActor` _array_element))
  (`KismetArrayLibrary.Array_Clear` _platforms))

(event `self.ReceiveBeginPlay`
  (bind _bitmap (`self.Bitmap`))
  (bind _width (`self.Width`))
  (while (> (- (`KismetMathLibrary.MultiplyMultiply_FloatFloat` 2.0 (`KismetMathLibrary.Conv_IntToDouble` (`KismetMathLibrary.Round` (* (`self.Width`) (.x (.scale (`self.GetTransform`))))))) 1.0) (`KismetMathLibrary.Conv_IntToDouble` _bitmap))
    (bind _freeindex (`self.Get Free Index` _bitmap))
    (bind _returnvalue (`|SpawnActorFromClass` (`KismetArrayLibrary.Array_Random` (`self.Generators`)) (`KismetMathLibrary.MakeTransform` (`KismetMathLibrary.MakeVector` (+ (.x (`self.K2_GetActorLocation`)) (* (/ _freeindex _width) 1000.0)) (+ (.y (`self.K2_GetActorLocation`)) (* (- (`KismetMathLibrary.Conv_IntToDouble` (mod _freeindex _width)) (/ (`KismetMathLibrary.Conv_IntToDouble` _width) 2.0)) 1000.0)) (+ (.z (`self.K2_GetActorLocation`)) 11.0))) "DontSpawnIfColliding" "OverrideRootScale" null null))
    (`/Engine/EditorBlueprintResources/StandardMacros.IsValid` _returnvalue
      (:`Is Valid`
        (`KismetArrayLibrary.Array_Add` (`self.Platforms`) _returnvalue)
        (bind _resultbitmap (`self.UpdateBitmap` (`self.Bitmap`) _returnvalue _freeindex))
        (set `self.Bitmap` _resultbitmap)))))

(fn `Get Free Index`
  (params (Bitmap :type Integer))
  (returns (FreeIndex :type Integer))
  (locals (TempBitmap :type Integer) (TempFreeIndex :type Integer))
  (bind _tempbitmap (`local.TempBitmap`))
  (set `local.TempBitmap` Bitmap)
  (set `local.TempFreeIndex` 0)
  (while (!= (mod _tempbitmap 2) 0)
    (set `local.TempBitmap` (/ _tempbitmap 2))
    (`/Engine/EditorBlueprintResources/StandardMacros.IncrementInt` (`local.TempFreeIndex`)))
  (return (`local.TempFreeIndex`)))

(fn `UpdateBitmap`
  (params (Bitmap :type Integer) (Actor :type "Actor Object Reference") (FreeIndex :type Integer))
  (returns (ResultBitmap :type Integer))
  (locals (Indices :type "Array of Integer") (TempBitmap :type Integer))
  (set `local.TempBitmap` Bitmap)
  (bind (_center _boxextent) (`GameplayStatics.GetActorArrayBounds` (`|MakeArray` Actor)))
  (for _index (range (`KismetMathLibrary.FTrunc` (/ (.x _boxextent) 500.0)))
    (for _index_2 (range (`KismetMathLibrary.FTrunc` (/ (.y _boxextent) 500.0)))
      (set `local.TempBitmap` (+ (`local.TempBitmap`) (`KismetMathLibrary.FTrunc` (`KismetMathLibrary.MultiplyMultiply_FloatFloat` 2.0 (`KismetMathLibrary.Conv_IntToDouble` (`KismetMathLibrary.Round` (+ (`KismetMathLibrary.Conv_IntToDouble` _index_2) (`KismetMathLibrary.Conv_IntToDouble` FreeIndex) (* (`self.Width`) (`KismetMathLibrary.Conv_IntToDouble` _index)))))))))))
  (return (`local.TempBitmap`)))

(fn `UserConstructionScript`)