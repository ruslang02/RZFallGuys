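; Game mode for a level-based platformer that handles failing, finishing and resetting levels, with a win after level 10 and a return to level 1 on failure.
; Fail and finish events pause play and show a message widget, notifying listeners through dispatchers.
; BeginPlay and Reset clear bonus effects, randomly reposition speed and passthrough pickups, place the ending platform and spawn random-length platforms with gaps that widen by level.
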(event `FailLevel`
  (bind _charactermovement (`Character.CharacterMovement` (`GameplayStatics.GetPlayerCharacter` 0)))
  (bind _output_get (set `self.Level` 1))
  (`self.OnLevelChanged` _output_get)
  (if (== (`self.InfoWidget`) null)
    (`self.SetActorHiddenInGame` (`GameplayStatics.GetPlayerPawn` 0) true)
    (set `CharacterMovementComponent.GravityScale` 0.0 _charactermovement)
    (`MovementComponent.StopMovementImmediately` _charactermovement)
    (bind _returnvalue (`|CreateWidget` "/Game/RZFallGuys/Blueprints/UI/FailLevelMessage.FailLevelMessage_C"))
    (bind _output_get_2 (set `self.InfoWidget` _returnvalue))
    (`UserWidget.AddToViewport` (stale `FinishLevel` _output_get_4) 0 :!label _label)
    (`UserWidget.AddToViewport` _output_get_2 0)
    (`UserWidget.AddToViewport` (stale `FinishLevel` _output_get_3) 0)
    (bind _output_get_3 (set `self.IsPaused` true))
    (`self.OnPausedChanged` _output_get_3)))

(event `Reset`
  (bind _dynamicactors (`self.DynamicActors`))
  (bind _returnvalue (+ (`self.Level`) 1))
  (`self.SetActorHiddenInGame` (`GameplayStatics.GetPlayerPawn` 0) false)
  (set `CharacterMovementComponent.GravityScale` 1.0 (`Character.CharacterMovement` (`GameplayStatics.GetPlayerCharacter` 0)))
  (bind _returnvalue_2 (`GameplayStatics.GetActorOfClass` "/Script/Engine.PlayerStart"))
  (`self.K2_SetActorLocation` (`GameplayStatics.GetPlayerPawn` 0) (`self.K2_GetActorLocation` _returnvalue_2) false true)
  (bind _output_get (set `self.IsPaused` false))
  (`self.OnPausedChanged` _output_get)
  (for _array_element _dynamicactors
    (`self.K2_DestroyActor` _array_element))
  (`KismetArrayLibrary.Array_Clear` _dynamicactors)
  (`self.InitVars` :!label _label_2)
  (set `self.Offset` 0.0)
  (set `self.ChunksCount` (`KismetMathLibrary.Conv_IntToDouble` _returnvalue))
  (`self.RepositionBonuses`)
  (bind _returnvalue_3 (`GameplayStatics.GetActorOfClass` "/Game/RZFallGuys/Blueprints/Platforms/EndingPlatform.EndingPlatform_C"))
  (`self.K2_SetActorTransform` _returnvalue_3 (`KismetMathLibrary.MakeTransform` (`KismetMathLibrary.MakeVector` (+ -7900.0 (* 1000.0 (+ (`KismetMathLibrary.Conv_IntToDouble` _returnvalue) 3.0))) 100.0) (struct :`Yaw` 90.0)) false true)
  (while (> (`self.ChunksCount`) 1.0) :!label _label_3
    (bind _returnvalue_4 (`|SpawnActorFromClass` "/Game/RZFallGuys/Blueprints/Platforms/GamePlatform.GamePlatform_C" (`KismetMathLibrary.MakeTransform` (`KismetMathLibrary.MakeVector` (+ (`self.Offset`) -5900.0) 100.0) (struct) (`KismetMathLibrary.MakeVector` (`KismetMathLibrary.Conv_IntToDouble` (`KismetMathLibrary.RandomIntegerInRange` 1 (`KismetMathLibrary.Min` (`KismetMathLibrary.FTrunc` (`self.ChunksCount`)) 4))) 1.0 1.0)) "AlwaysSpawn" "OverrideRootScale" null null))
    (`KismetArrayLibrary.Array_Add` (`self.DynamicActors`) _returnvalue_4)
    (bind _returnvalue_5 (+ (.x (`self.GetActorScale3D` _returnvalue_4)) 0.5 (* (`KismetMathLibrary.Conv_IntToDouble` (`self.Level`)) 0.01)))
    (set `self.ChunksCount` (- (`self.ChunksCount`) _returnvalue_5))
    (set `self.Offset` (+ (* 1000 _returnvalue_5) (`self.Offset`)))
    (goto _label_3)))

(event `FinishLevel`
  (bind _output_get (set `self.Level` (+ (`self.Level`) 1)))
  (`self.OnLevelChanged` _output_get)
  (if (and (== (`self.InfoWidget`) null) (not (`self.IsPaused`)))
    (`MovementComponent.StopMovementImmediately` (`Character.CharacterMovement` (`GameplayStatics.GetPlayerCharacter` 0)))
    (if (== _output_get 11)
      (bind _returnvalue (`|CreateWidget` "/Game/RZFallGuys/Blueprints/UI/WinGameMessage.WinGameMessage_C"))
      (bind _output_get_2 (set `self.Level` 1))
      (`self.OnLevelChanged` _output_get_2)
      (bind _output_get_3 (set `self.InfoWidget` _returnvalue))
      (goto _label)
      (else
        (bind _returnvalue_2 (`|CreateWidget` "/Game/RZFallGuys/Blueprints/UI/WinLevelMessage.WinLevelMessage_C"))
        (bind _output_get_4 (set `self.InfoWidget` _returnvalue_2))
        (goto _label)))))

(event `self.ReceiveBeginPlay`
  (goto _label_2))

(fn `InitVars`
  (bind _output_get (set `self.SpeedMultiplier` 1.0))
  (`self.OnSpeedChanged` _output_get)
  (bind _output_get_2 (set `self.IsPassthrough` false))
  (`self.OnPassthroughChanged` _output_get_2))

(fn `RepositionBonuses`
  (bind _returnvalue (`KismetMathLibrary.MakeVector` (`KismetMathLibrary.RandomFloatInRange` -5500.0 (+ (* 1000 (`self.ChunksCount`)) -6500.0)) (`KismetMathLibrary.RandomFloatInRange` -1400.0 1400.0)))
  (bind _returnvalue_2 (`GameplayStatics.GetActorOfClass` "/Game/RZFallGuys/Blueprints/Bonuses/SpeedBonus.SpeedBonus_C"))
  (`self.K2_SetActorLocation` _returnvalue_2 _returnvalue false false)
  (bind _returnvalue_3 (`GameplayStatics.GetActorOfClass` "/Game/RZFallGuys/Blueprints/Bonuses/PassthroughBonus.PassthroughBonus_C"))
  (`self.K2_SetActorLocation` _returnvalue_3 _returnvalue false false))

(fn `UserConstructionScript`)