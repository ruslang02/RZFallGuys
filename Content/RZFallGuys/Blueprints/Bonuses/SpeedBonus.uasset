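; SpeedBonus is a pickup that temporarily lowers the game mode's speed multiplier when the first player's pawn touches it.
; On sphere overlap it hides, disables overlaps, broadcasts the reduced multiplier through RzGameMode, then restores and rebroadcasts normal speed after a retriggerable delay.
; It binds to the game mode's pause-changed event and becomes visible and collectible again whenever the game unpauses, rather than respawning on a timer.
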(event `OnPausedChanged`
  (params (Paused :type Boolean))
  (if (not Paused)
    (`self.SetActorHiddenInGame` false)
    (set `PrimitiveComponent.bGenerateOverlapEvents` true (`self.Sphere`))))

(event `self.ReceiveBeginPlay`
  (bind _asrz_game_mode (cast `/Game/RZFallGuys/Blueprints/RzGameMode` (`GameplayStatics.GetGameMode`)))
  (add `/Game/RZFallGuys/Blueprints/RzGameMode.OnPausedChanged` _asrz_game_mode (delegate `OnPausedChanged`)))

(event `self.Sphere.OnComponentBeginOverlap`
  (params (OverlappedComponent :type "PrimitiveComponent Object Reference") (OtherActor :type "Actor Object Reference") (OtherComp :type "PrimitiveComponent Object Reference") (OtherBodyIndex :type Integer) (bFromSweep :type Boolean) (SweepResult :type "HitResult Structure (by ref)"))
  (if (== OtherActor (`GameplayStatics.GetPlayerPawn` 0))
    (`self.SetActorHiddenInGame` true)
    (set `PrimitiveComponent.bGenerateOverlapEvents` false (`self.Sphere`))
    (bind _asrz_game_mode (cast `/Game/RZFallGuys/Blueprints/RzGameMode` (`GameplayStatics.GetGameMode`)))
    (bind _output_get (set `/Game/RZFallGuys/Blueprints/RzGameMode.SpeedMultiplier` 0.3 _asrz_game_mode))
    (`/Game/RZFallGuys/Blueprints/RzGameMode.OnSpeedChanged` _asrz_game_mode _output_get)
    (`KismetSystemLibrary.RetriggerableDelay` 10.0)
    (bind _output_get_2 (set `/Game/RZFallGuys/Blueprints/RzGameMode.SpeedMultiplier` 1.0 _asrz_game_mode))
    (`/Game/RZFallGuys/Blueprints/RzGameMode.OnSpeedChanged` _asrz_game_mode _output_get_2)))

(fn `UserConstructionScript`)